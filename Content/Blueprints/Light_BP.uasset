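; Light Blueprint with a spotlight that the player can switch on and off with the F key while input is enabled by its trigger.
; Any overlap with the trigger enables input for player 0 and ending it disables input, both flipping the help text's visibility without checking the overlapping actor.
; The construction script applies the light color and starting visibility from variables.
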(event `self.Trigger.OnComponentBeginOverlap`
  (params (OverlappedComponent :type "PrimitiveComponent Object Reference") (OtherActor :type "Actor Object Reference") (OtherComp :type "PrimitiveComponent Object Reference") (OtherBodyIndex :type Integer) (bFromSweep :type Boolean) (SweepResult :type "HitResult Structure (by ref)"))
  ;[0.0625 0.1698 1] When overlapping trigger, enable input and show helpful text.  Disable when leaving.
  (`self.EnableInput` (`GameplayStatics.GetPlayerController` 0))
  (`SceneComponent.ToggleVisibility` (`self.HelpfulText`) false :!label _label))

(event `self.Trigger.OnComponentEndOverlap`
  (params (OverlappedComponent :type "PrimitiveComponent Object Reference") (OtherActor :type "Actor Object Reference") (OtherComp :type "PrimitiveComponent Object Reference") (OtherBodyIndex :type Integer))
  ;[0.0625 0.1698 1] When overlapping trigger, enable input and show helpful text.  Disable when leaving.
  (`self.DisableInput` (`GameplayStatics.GetPlayerController` 0))
  (goto _label))

(event `Key|F`
  (params (Key :type "Key Structure"))
  ;[1 0.6014 0.1729] Comment
  (:`Pressed`
    (`SceneComponent.ToggleVisibility` (`self.SpotLight`) false)))

(fn `UserConstructionScript`
  (bind _spotlight (`self.SpotLight`))
  (`LightComponent.SetLightColor` _spotlight (`self.Light Color`) true)
  (`SceneComponent.SetVisibility` _spotlight (`self.Visibility Setting`) false))